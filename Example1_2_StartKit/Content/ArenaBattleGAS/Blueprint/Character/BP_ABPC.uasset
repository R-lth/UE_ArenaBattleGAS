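; BP_ABPC is a character Blueprint for the ArenaBattle GAS game that sets up the player's HUD and reacts to the game being cleared.
; On possession it creates WBP_HUD for player controllers only, then separately binds a gameplay tag-change wrapper on its ASC for Event.Game.Cleared.
; Any change to that tag's presence calls SetGameCleared on the HUD and activates the GameCleared component, without checking the tag count.
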(event Custom|OnGameplayTagChangeBP
  (params (Tag :type Gameplay%20Tag%20Structure%20%28by%20ref%29) (TagCount :type Integer))
  (Default|SetGameCleared (Variables|Default|GetHUDWidget)) ; HUDWidget 안에 있는 Set Game Cleared
  (Components|Activation|Activate (Variables|Default|GetGameCleared) false) ; 발동
)

(event EventBeginPlay)

(event EventPossessed
  (params (NewController :type Controller%20Object%20Reference))
  (Utilities|FlowControl|Sequence ; HUD 생성 로직과 바인딩 로직을 분리
    (:then_0
      (if (Class|Controller|IsPlayerController NewController) ; 플레이어면 true. 아니면 false
        (bind _returnvalue (UserInterface|CreateWidget "/Game/ArenaBattleGAS/UI/WBP_HUD.WBP_HUD_C"))
        (bind _output_get (Variables|Default|SetHUDWidget _returnvalue))
        (UserInterface|Viewport|AddtoViewport _output_get 0)))
    (:then_1
      (GameplayTags|BindEventWrappertoGameplayTagChanged (Variables|Default|GetASC) "(TagName=\"Event.Game.Cleared\")" (delegate Custom|OnGameplayTagChangeBP)) ; 게임플레이 태그가 바뀔 때 이벤트가 호출된다
    )))

(fn ConstructionScript)