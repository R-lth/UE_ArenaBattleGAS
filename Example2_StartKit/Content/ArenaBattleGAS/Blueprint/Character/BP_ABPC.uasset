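; BP_ABPC is the player character Blueprint, connecting input and UI to the Gameplay Ability System.
; On possession by a player controller it creates the WBP_HUD widget and turns on the ability system debug display.
; IA_Attack activates abilities by the Character.Action.Attack tag.
; A callback bound to the Event.Game.Cleared tag change activates the GameCleared component and sets the HUD to its cleared state.
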(event Custom|OnGameClearedBP
  (params (Tag :type Gameplay%20Tag%20Structure%20%28by%20ref%29) (TagCount :type Integer))
  ;[0.15 0.15 0.15 0.5] Comment
  (Components|Activation|Activate (Variables|Default|GetGameCleared) false)
  (Default|SetGameCleared (Variables|Default|GetHUDWidget)))

(event Input|EnhancedActionEvents|EnhancedInputActionIA_Attack
  (params (ActionValue :type Boolean) (ElapsedSeconds :type Float%20%28double-precision%29) (TriggeredSeconds :type Float%20%28double-precision%29) (InputAction :type Input%20Action%20Object%20Reference :default "/Game/ArenaBattle/Input/Actions/IA_Attack.IA_Attack"))
  ;[0.15 0.15 0.15 0.5] Comment
  (Abilities|TryActivateAbilitiesbyTag (Variables|Default|GetASC) (GameplayTags|MakeGameplayTagContainerfromTag "(TagName=\"Character.Action.Attack\")") true))

(event EventBeginPlay
  ;[0.15 0.15 0.15 0.5] Comment
  (GameplayTags|BindEventWrappertoGameplayTagChanged (Variables|Default|GetASC) "(TagName=\"Event.Game.Cleared\")" (delegate Custom|OnGameClearedBP)))

(event EventPossessed
  (params (NewController :type Controller%20Object%20Reference))
  ;[0.15 0.15 0.15 0.5] GAS
  (Utilities|FlowControl|Sequence
    (:then_0
      (if (Class|Controller|IsPlayerController NewController)
        (bind _returnvalue (UserInterface|CreateWidget "/Game/ArenaBattleGAS/UI/WBP_HUD.WBP_HUD_C"))
        (bind _output_get (Variables|Default|SetHUDWidget _returnvalue))
        (UserInterface|Viewport|AddtoViewport _output_get 0)
        (Development|ExecuteConsoleCommand "showdebug abilitysystem" 0)))))

(fn ConstructionScript)